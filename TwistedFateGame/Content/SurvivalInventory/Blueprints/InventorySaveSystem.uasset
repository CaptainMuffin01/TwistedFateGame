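; Server-driven save actor for the survival inventory game, persisting living players' stats and equipment, world items and storage containers to one InventorySave slot.
; An optional looping timer rebuilds and writes the save.
; Shortly after BeginPlay, saved items replace placed ones through multicast respawning.
; Players and storage are looked up by name on request; player-entry deletion edits only the loaded object, while a multicast event deletes the whole slot.
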(event Custom|Server%20Set%20Auto%20Save%20Timer
  ;[1 1 1] Server set auto save
  ;;[1 1 1] Server set auto save timer
  ;;[1 1 1] Auto save
  (if (Variables|SaveSettings|AutoSave|GetAuto%20Save)
    ;;[1 1 1] Set event by timer
    (Utilities|Time|SetTimerbyEvent (delegate Custom|Server%20Auto%20Save) (Variables|SaveSettings|AutoSave|GetAuto%20Save%20Timer) true)))

(event Custom|Multicast%20Delete%20Save
  ;[1 1 1] Multicast delete save
  (SaveGame|DeleteGameinSlot (Variables|SaveSettings|Loading|GetSave%20Name)))

(event Custom|Server%20Load%20Items
  ;[1 1 1] Server load items
  (bind _returnvalue (SaveGame|LoadGamefromSlot (Variables|SaveSettings|Loading|GetSave%20Name)))
  (bind _asinventory_save (Utilities|Casting|CastToInventorySave _returnvalue))
  (CallFunction|LoadItems _asinventory_save))

(event Custom|Server%20Auto%20Save
  ;[1 1 1] Server auto save
  ;;[1 1 1] Server auto save
  ;;[1 1 1] Create game object
  (bind _returnvalue (SaveGame|CreateSaveGameObject "/Game/SurvivalInventory/Blueprints/InventorySave.InventorySave_C"))
  ;;[1 1 1] Save player stats
  (CallFunction|SavePlayerStats _returnvalue)
  ;;[1 1 1] Save items
  (CallFunction|SaveItems _returnvalue)
  ;;[1 1 1] Save storage component
  (CallFunction|SaveStorageComponents _returnvalue))

(event Custom|Multicast%20Spawn%20Items
  (params (Item%20Save :type S%20Item%20Save%20Structure))
  ;[1 1 1] Multicast spawn item
  (bind _returnvalue (Game|SpawnActorfromClass "/Game/SurvivalInventory/Blueprints/Items/Item.Item_C" (.transform Item%20Save) "AdjustIfPossibleButAlwaysSpawn" 0 (.item Item%20Save) 0))
  (Default|OnSpawned _returnvalue))

(event EventBeginPlay
  ;[1 1 1] Begin Play
  ;;[1 1 1] Server start auto save timer
  (CallFunction|ServerSetAutoSaveTimer)
  ;;[1 1 1] Delay
  (Utilities|FlowControl|Delay 1.0)
  ;;[1 1 1] Call server load items
  (CallFunction|ServerLoadItems))

(fn ConstructionScript)

(fn SavePlayerStats
  (params (Inventory%20Save :type Inventory%20Save%20Object%20Reference))
  ;[1 1 1] Save player stats
  ;;[1 1 1] Set local
  (LocalVariables|SetSave%20Object%20L Inventory%20Save)
  ;;[1 1 1] Debug text
  (CallFunction|DebugText "Saving Player Stats...")
  ;;[1 1 1] Clear save
  (Utilities|Array|Clear (Variables|/Game/SurvivalInventory/Blueprints/InventorySave.InventorySave_C|GetInventory%20Component%20Saves (LocalVariables|GetSave%20Object%20L)))
  ;;[1 1 1] Get all players
  (bind _outactors (Actor|GetAllActorsOfClass "/Game/RifleAnimsetPro/Survivor/Hero_BP.Hero_BP_C"))
  (for _array_element _outactors
    ;;[1 1 1] Set component
    (bind _output_get (LocalVariables|SetPlayer%20Inventory%20Component%20L (Variables|/Game/RifleAnimsetPro/Survivor/Hero_BP.Hero_BP_C|GetPlayerInventoryComponent _array_element)))
    (Utilities|IsValid _output_get
      (:Is%20Valid
        ;;[1 1 1] Is player alive
        (if (not (Variables|/Game/SurvivalInventory/Blueprints/Components/PlayerInventoryComponent.PlayerInventoryComponent_C|GetPlayer%20Dead _output_get))
          ;;[1 1 1] Save all inventory component stats
          (Utilities|Array|Add (Variables|/Game/SurvivalInventory/Blueprints/InventorySave.InventorySave_C|GetInventory%20Component%20Saves (LocalVariables|GetSave%20Object%20L)) (Utilities|Struct|MakeS_PlayerSave (Variables|/Game/SurvivalInventory/Blueprints/Components/PlayerInventoryComponent.PlayerInventoryComponent_C|GetPlayer%20Name (LocalVariables|GetPlayer%20Inventory%20Component%20L)) (Variables|/Game/SurvivalInventory/Blueprints/Components/MasterInventoryComponent.MasterInventoryComponent_C|GetInventory%20Slots (LocalVariables|GetPlayer%20Inventory%20Component%20L)) (Variables|/Game/SurvivalInventory/Blueprints/Components/PlayerInventoryComponent.PlayerInventoryComponent_C|GetHealth (LocalVariables|GetPlayer%20Inventory%20Component%20L)) (Variables|/Game/SurvivalInventory/Blueprints/Components/PlayerInventoryComponent.PlayerInventoryComponent_C|GetHunger (LocalVariables|GetPlayer%20Inventory%20Component%20L)) (Variables|/Game/SurvivalInventory/Blueprints/Components/PlayerInventoryComponent.PlayerInventoryComponent_C|GetThirst (LocalVariables|GetPlayer%20Inventory%20Component%20L)) (Variables|/Game/SurvivalInventory/Blueprints/Components/MasterInventoryComponent.MasterInventoryComponent_C|GetInventory (LocalVariables|GetPlayer%20Inventory%20Component%20L)) (Variables|/Game/SurvivalInventory/Blueprints/Components/PlayerInventoryComponent.PlayerInventoryComponent_C|GetHead%20Equipment%20Slot (LocalVariables|GetPlayer%20Inventory%20Component%20L)) (Variables|/Game/SurvivalInventory/Blueprints/Components/PlayerInventoryComponent.PlayerInventoryComponent_C|GetChest%20Equipment%20Slot (LocalVariables|GetPlayer%20Inventory%20Component%20L)) (Variables|/Game/SurvivalInventory/Blueprints/Components/PlayerInventoryComponent.PlayerInventoryComponent_C|GetLegs%20Equipment%20Slot (LocalVariables|GetPlayer%20Inventory%20Component%20L)) (Variables|/Game/SurvivalInventory/Blueprints/Components/PlayerInventoryComponent.PlayerInventoryComponent_C|GetBackpack%20Equipment%20Slot (LocalVariables|GetPlayer%20Inventory%20Component%20L)) (Variables|/Game/SurvivalInventory/Blueprints/Components/PlayerInventoryComponent.PlayerInventoryComponent_C|GetFeet%20Equipment%20Slot (LocalVariables|GetPlayer%20Inventory%20Component%20L)) (Transformation|GetActorTransform (Variables|/Game/SurvivalInventory/Blueprints/Components/PlayerInventoryComponent.PlayerInventoryComponent_C|GetHero (LocalVariables|GetPlayer%20Inventory%20Component%20L))) (Variables|/Game/SurvivalInventory/Blueprints/Components/PlayerInventoryComponent.PlayerInventoryComponent_C|GetHeld%20Item (LocalVariables|GetPlayer%20Inventory%20Component%20L)) (Variables|/Game/SurvivalInventory/Blueprints/Components/MasterInventoryComponent.MasterInventoryComponent_C|GetWeight (LocalVariables|GetPlayer%20Inventory%20Component%20L)) (Variables|/Game/SurvivalInventory/Blueprints/Components/MasterInventoryComponent.MasterInventoryComponent_C|GetMax%20Weight (LocalVariables|GetPlayer%20Inventory%20Component%20L))))))))
  ;;[1 1 1] Save game
  (bind _returnvalue (SaveGame|SaveGametoSlot (LocalVariables|GetSave%20Object%20L) (Variables|SaveSettings|Loading|GetSave%20Name)))
  ;;[1 1 1] Debug text
  (if _returnvalue
    (CallFunction|DebugText "Player Stats Saved")
    (else
      (CallFunction|DebugText "Player Stats Error"))))

(fn DebugText
  (params (Debug%20Text :type String))
  (LocalVariables|SetDebug%20Text%20L Debug%20Text)
  ;[1 1 1] Show grid debug text
  (if (Variables|SaveSettings|Debug|GetShow%20Debug%20Text)
    ;[1 1 1] Print to screen
    (Development|PrintString (LocalVariables|GetDebug%20Text%20L) true true "(R=0.000000,G=0.660000,B=1.000000,A=1.000000)" (Variables|SaveSettings|Debug|GetDebug%20Text%20Time))))

(fn FindPlayerSave
  (params (Player%20Name :type String))
  ;[1 1 1] Find player save
  ;;[1 1 1] Set local
  (LocalVariables|SetPlayer%20Name%20L Player%20Name)
  ;;[1 1 1] Load save
  (bind _returnvalue (SaveGame|LoadGamefromSlot (Variables|SaveSettings|Loading|GetSave%20Name)))
  (bind _asinventory_save (Utilities|Casting|CastToInventorySave _returnvalue))
  (LocalVariables|SetLoaded%20Save%20L _asinventory_save)
  ;;[1 1 1] Loop through saves to find player save
  (bind _array_element (Utilities|Array|ForEachLoopwithBreak (Variables|/Game/SurvivalInventory/Blueprints/InventorySave.InventorySave_C|GetInventory%20Component%20Saves (LocalVariables|GetLoaded%20Save%20L)) :!label _label)
    (:LoopBody
      ;;[1 1 1] If matching names set inventory save
      (if (Utilities|Enum|Equal(Enum) (Utilities|Struct|BreakS_PlayerSave _array_element) (LocalVariables|GetPlayer%20Name%20L))
        (LocalVariables|SetInventory%20Save%20L _array_element)
        (LocalVariables|SetReturn%20Value%20L true)
        (goto _label Break)))
    (:Completed
      ;;[1 1 1] Is save found
      (if (LocalVariables|GetReturn%20Value%20L)
        (return true (LocalVariables|GetInventory%20Save%20L))
        (else
          (return false ""))))))

(fn SaveItems
  (params (Inventory%20Save :type Inventory%20Save%20Object%20Reference))
  ;[1 1 1] Save items
  ;;[1 1 1] Set local
  (LocalVariables|SetSave%20Object Inventory%20Save)
  ;;[1 1 1] Debug text
  (CallFunction|DebugText "Saving Items...")
  ;;[1 1 1] Clear save
  (Utilities|Array|Clear (Variables|/Game/SurvivalInventory/Blueprints/InventorySave.InventorySave_C|GetItem%20Saves (LocalVariables|GetSave%20Object)))
  ;;[1 1 1] Get all items and loop them
  (bind _outactors (Actor|GetAllActorsOfClass "/Game/SurvivalInventory/Blueprints/Items/Item.Item_C"))
  (for _array_element _outactors
    (LocalVariables|SetItem%20L _array_element)
    ;;[1 1 1] Add item to save game item array
    (Utilities|Array|Add (Variables|/Game/SurvivalInventory/Blueprints/InventorySave.InventorySave_C|GetItem%20Saves (LocalVariables|GetSave%20Object)) (Utilities|Struct|MakeS_ItemSave (Variables|/Game/SurvivalInventory/Blueprints/Items/Item.Item_C|GetItem (LocalVariables|GetItem%20L)) (Transformation|GetWorldTransform (Variables|/Game/SurvivalInventory/Blueprints/Items/Item.Item_C|GetItem%20World%20Mesh (LocalVariables|GetItem%20L))))))
  ;;[1 1 1] Save game
  (SaveGame|SaveGametoSlot (LocalVariables|GetSave%20Object) (Variables|SaveSettings|Loading|GetSave%20Name)))

(fn LoadItems
  (params (Inventory%20Save :type Inventory%20Save%20Object%20Reference))
  ;[1 1 1] Load items
  ;;[1 1 1] Set local
  (LocalVariables|SetSave%20Object%20L Inventory%20Save)
  ;;[1 1 1] Destory all start items
  (bind _outactors (Actor|GetAllActorsOfClass "/Game/SurvivalInventory/Blueprints/Items/Item.Item_C"))
  (for _array_element _outactors
    (Actor|DestroyActor _array_element))
  ;;[1 1 1] Loop for each item in save array
  (for _array_element_2 (Variables|/Game/SurvivalInventory/Blueprints/InventorySave.InventorySave_C|GetItem%20Saves (LocalVariables|GetSave%20Object%20L))
    (LocalVariables|SetItem%20Save%20L _array_element_2)
    ;;[1 1 1] Multicast spawn item
    (CallFunction|MulticastSpawnItems (LocalVariables|GetItem%20Save%20L))))

(fn SaveStorageComponents
  (params (Inventory%20Save :type Inventory%20Save%20Object%20Reference))
  ;[1 1 1] Save storage components
  ;;[1 1 1] Set local
  (LocalVariables|SetSave%20Object Inventory%20Save)
  ;;[1 1 1] Clear save
  (Utilities|Array|Clear (Variables|/Game/SurvivalInventory/Blueprints/InventorySave.InventorySave_C|GetStorage%20Component%20Saves (LocalVariables|GetSave%20Object)))
  ;;[1 1 1] Debug text
  (CallFunction|DebugText "Saving Storage...")
  ;;[1 1 1] Get all master storage actors
  (bind _outactors (Actor|GetAllActorsOfClass "/Game/SurvivalInventory/Blueprints/MasterStorage.MasterStorage_C"))
  (for _array_element _outactors
    ;;[1 1 1] Set array storage component
    (LocalVariables|SetStorage%20Component%20L (Variables|/Game/SurvivalInventory/Blueprints/MasterStorage.MasterStorage_C|GetStorageInventoryComponent _array_element))
    ;;[1 1 1] Save storage stats to save object
    (Utilities|Array|Add (Variables|/Game/SurvivalInventory/Blueprints/InventorySave.InventorySave_C|GetStorage%20Component%20Saves (LocalVariables|GetSave%20Object)) (Utilities|Struct|MakeS_StorageSave (Variables|/Game/SurvivalInventory/Blueprints/Components/StorageInventoryComponent.StorageInventoryComponent_C|GetName (LocalVariables|GetStorage%20Component%20L)) (Variables|/Game/SurvivalInventory/Blueprints/Components/MasterInventoryComponent.MasterInventoryComponent_C|GetInventory (LocalVariables|GetStorage%20Component%20L)) (Variables|/Game/SurvivalInventory/Blueprints/Components/MasterInventoryComponent.MasterInventoryComponent_C|GetWeight (LocalVariables|GetStorage%20Component%20L)) (Variables|/Game/SurvivalInventory/Blueprints/Components/MasterInventoryComponent.MasterInventoryComponent_C|GetInventory%20Slots (LocalVariables|GetStorage%20Component%20L)))))
  ;;[1 1 1] Save game
  (SaveGame|SaveGametoSlot (LocalVariables|GetSave%20Object) (Variables|SaveSettings|Loading|GetSave%20Name)))

(fn LoadStorageComponent
  (params (Storage%20Name :type String))
  ;[1 1 1] Load storage component
  ;;[1 1 1] Set local
  (LocalVariables|SetStorage%20Name%20L Storage%20Name)
  ;;[1 1 1] Load save game
  (bind _returnvalue (SaveGame|LoadGamefromSlot (Variables|SaveSettings|Loading|GetSave%20Name)))
  (bind _asinventory_save (Utilities|Casting|CastToInventorySave _returnvalue))
  (bind _output_get (LocalVariables|SetLoaded%20Save%20L _asinventory_save))
  ;;[1 1 1] Loop for storage component saves
  (bind _array_element (Utilities|Array|ForEachLoopwithBreak (Variables|/Game/SurvivalInventory/Blueprints/InventorySave.InventorySave_C|GetStorage%20Component%20Saves _output_get) :!label _label)
    (:LoopBody
      ;;[1 1 1] Check if names match
      (if (Utilities|Enum|Equal(Enum) (Utilities|Struct|BreakS_StorageSave _array_element) (LocalVariables|GetStorage%20Name%20L))
        ;;[1 1 1] If true set storage save
        (LocalVariables|SetStorage%20Save%20L _array_element)
        (LocalVariables|SetReturn%20Value%20L true)
        (goto _label Break)))
    (:Completed
      ;;[1 1 1] Return storage save
      (if (LocalVariables|GetReturn%20Value%20L)
        (return true (LocalVariables|GetStorage%20Save%20L))
        (else
          (return false ""))))))

(fn DeletePlayerSave
  (params (Player%20Name :type String))
  ;[1 1 1] Delete player save
  ;;[1 1 1] Set local
  (LocalVariables|SetPlayer%20Name%20L Player%20Name)
  ;;[1 1 1] Get save game
  (bind _returnvalue (SaveGame|LoadGamefromSlot (Variables|SaveSettings|Loading|GetSave%20Name)))
  (bind _asinventory_save (Utilities|Casting|CastToInventorySave _returnvalue))
  (bind _output_get (LocalVariables|SetGame%20Save%20L _asinventory_save))
  ;;[1 1 1] Loop through player saves
  (bind _array_element (Utilities|Array|ForEachLoopwithBreak (Variables|/Game/SurvivalInventory/Blueprints/InventorySave.InventorySave_C|GetInventory%20Component%20Saves _output_get) :!label _label)
    (:LoopBody
      ;;[1 1 1] Check if names match
      (if (Utilities|Enum|Equal(Enum) (.PlayerName (Utilities|Struct|BreakS_PlayerSave _array_element)) (LocalVariables|GetPlayer%20Name%20L))
        ;;[1 1 1] If true remove from save array
        (LocalVariables|SetReturn%20Value%20L true)
        (Utilities|Array|RemoveItem (Variables|/Game/SurvivalInventory/Blueprints/InventorySave.InventorySave_C|GetInventory%20Component%20Saves (LocalVariables|GetGame%20Save%20L)) _array_element)
        (goto _label Break)))
    (:Completed
      ;;[1 1 1] Return value
      (return (LocalVariables|GetReturn%20Value%20L)))))