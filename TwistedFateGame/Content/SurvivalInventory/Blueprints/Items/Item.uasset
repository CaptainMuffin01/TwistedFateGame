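; World item actor for a survival inventory, representing a pickup with an item ID and count.
; The construction script builds the item struct from the selected data table row, or resets the selection from the struct's ID if the lookup fails, then applies the world mesh.
; OnSpawned syncs selection, count and mesh from the item struct.
; Interact passes the actor to the player component's ServerPickupItem, while DestroyItem removes it for all clients.
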(event Custom|Destroy%20Item
  ;[1 1 1] All clients destroy item
  (Actor|DestroyActor))

(event Custom|On%20Spawned
  (bind _item (Variables|Default|GetItem))
  (bind (_id _count) (Utilities|Struct|BreakS_Item _item))
  ;[1 1 1] On spawned
  ;;[1 1 1] Set selected item
  (Variables|Default|SetSelect%20Item (Utilities|Struct|MakeDataTableRowHandle "/Game/SurvivalInventory/Blueprints/Items/ItemData.ItemData" (Utilities|String|StringToName _id)))
  (Variables|Default|SetCount _count)
  ;;[1 1 1] Set static mesh
  (Components|StaticMesh|SetStaticMesh (Variables|Default|GetItem%20World%20Mesh) (Utilities|Struct|BreakS_ItemDetails (.Item%20Details%20Out (CallFunction|ItemDetails (Variables|Default|GetItem))))))

(event EventInteract
  (params (Player%20Component :type Player%20Inventory%20Component%20Object%20Reference))
  ;[1 1 1] Server calls interact
  (Default|ServerPickupItem Player%20Component self))

(fn ConstructionScript
  (if (.Return%20Value (CallFunction|ItemDetails (Utilities|Struct|MakeS_Item (Utilities|String|ToString(Name) (.RowName (Utilities|Struct|BreakDataTableRowHandle (Variables|Default|GetSelect%20Item)))) 0 0 0)))
    (Variables|Default|SetItem (Utilities|Struct|MakeS_Item (Utilities|String|ToString(Name) (.RowName (Utilities|Struct|BreakDataTableRowHandle (Variables|Default|GetSelect%20Item)))) (Variables|Default|GetCount) 0 0))
    (else
      (Variables|Default|SetSelect%20Item (Utilities|Struct|MakeDataTableRowHandle "/Game/SurvivalInventory/Blueprints/Items/ItemData.ItemData" (Utilities|String|StringToName (.id (Variables|Default|GetItem)))))))
  (if (.Return%20Value (CallFunction|ItemDetails (Variables|Default|GetItem)))
    (Components|StaticMesh|SetStaticMesh (Variables|Default|GetItem%20World%20Mesh) (.WorldMesh (Utilities|Struct|BreakS_ItemDetails (.Item%20Details%20Out (CallFunction|ItemDetails (Variables|Default|GetItem))))))))