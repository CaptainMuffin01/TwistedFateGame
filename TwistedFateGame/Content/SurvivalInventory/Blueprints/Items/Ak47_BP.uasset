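; AK-47 weapon Blueprint for the survival inventory game, providing automatic fire through trigger pull and release events.
; A DoOnce-gated pull fires immediately and starts a looping timer at RoundsPerSecond, which release clears.
; Each shot spawns a Bullet_BP, sound and muzzle effect, decrements Hero_BP's magazine count and removes one 7.62 round from the player's inventory.
; Fire itself performs no ammo check.
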(event Custom|Fire
  (Game|SpawnActorfromClass "/Game/RifleAnimsetPro/Weapons/Bullet_BP.Bullet_BP_C" (Transformation|GetWorldTransform (Variables|Default|GetBullet%20Spawn)) "Undefined" 0 0)
  (Audio|PlaySound2D "/Game/RifleAnimsetPro/Weapons/Sounds/ak74_shot_1.ak74_shot_1")
  (Effects|SpawnEmitteratLocation "/Game/IBWP3DArK47/Particles/PS_VFX_ArK47.PS_VFX_ArK47" (Transformation|GetSocketLocation (Variables|Default|GetAK47) "Fire_FX_Slot") (Transformation|GetSocketRotation (Variables|Default|GetAK47) "Fire_FX_Slot"))
  (bind _ashero_bp (Utilities|Casting|CastToHero_BP (Game|GetPlayerCharacter 0)))
  (Math|Integer|DecrementInt (Variables|/Game/RifleAnimsetPro/Survivor/Hero_BP.Hero_BP_C|GetAmmoInMag%20AK47 _ashero_bp)
    (:%20%20
      (bind _item_count (Default|GetItemCount (Variables|/Game/RifleAnimsetPro/Survivor/Hero_BP.Hero_BP_C|GetPlayerInventoryComponent _ashero_bp)))
      (bind _item (Default|SearchforItem (Variables|/Game/RifleAnimsetPro/Survivor/Hero_BP.Hero_BP_C|GetPlayerInventoryComponent _ashero_bp) "7.62Rounds" _item_count false))
      (Default|RemoveItem (Variables|/Game/RifleAnimsetPro/Survivor/Hero_BP.Hero_BP_C|GetPlayerInventoryComponent _ashero_bp) _item false 1))))

(event EventTick
  (params (DeltaSeconds :type Float%20%28single-precision%29)))

(event EventTriggerPullBPI
  (Utilities|FlowControl|DoOnce false
    (:Completed
      (CallFunction|Fire)
      (Utilities|Time|SetTimerbyFunctionName 0 "Fire" (/ 1.0 (Variables|Default|GetRounds%20Per%20Second)) true))))

(event EventReleaseTriggerBPI
  (Utilities|Time|ClearTimerbyFunctionName 0 "Fire")
  (Utilities|FlowControl|DoOnce false) ; enters at Reset
)

(fn ConstructionScript
  (|CallParentFunction))