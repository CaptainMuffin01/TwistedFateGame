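; Model viewer actor for the survival inventory that renders a preview of the equipped character and of a single static mesh to two render textures.
; Equipment updates swap the skeletal mesh for the matching slot, with head, chest, legs, feet and backpack following the body's pose via master pose component.
; The viewed mesh can be set, rotated or hidden, and is rescaled from its bounds to a desired radius, capped at a maximum scale.
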(event Custom|On%20Spawned
  ;[1 1 1] Set render textures
  (Variables|/Script/Engine.SceneCaptureComponent2D|SetTextureTarget (Variables|Default|GetCaptureComponent) "/Game/SurvivalInventory/Blueprints/ModelViewer/RT_ModelViewerOutput.RT_ModelViewerOutput")
  (Variables|/Script/Engine.SceneCaptureComponent2D|SetTextureTarget (Variables|Default|GetSceneCaptureComponent2D) "/Game/SurvivalInventory/Blueprints/ModelViewer/RT_ModelViewerOutput2.RT_ModelViewerOutput2"))

(event Custom|Update%20Character%20Equipment
  (params (Equipment%20Slot :type S%20Equipment%20Slot%20Structure))
  (bind (_slottype _equipteditem) (Utilities|Struct|BreakS_EquipmentSlot Equipment%20Slot))
  ;[1 1 1] Update model viewer character
  (Class|SkinnedMeshComponent|SetSkeletalMesh (Utilities|Select :Index _slottype :NewEnumerator0 0 :NewEnumerator1 (Variables|Default|GetBackpack) :NewEnumerator2 (Variables|Default|GetFeet) :NewEnumerator3 (Variables|Default|GetHead) :NewEnumerator4 (Variables|Default|GetChest) :NewEnumerator5 (Variables|Default|GetLegs) :NewEnumerator8 (Variables|Default|GetRight%20Hand)) (Utilities|Struct|BreakS_ItemDetails (.Item%20Details%20Out (CallFunction|ItemDetails _equipteditem))) true))

(fn ConstructionScript
  (bind _skeletalmesh (Variables|Default|GetSkeletalMesh))
  (Class|SkinnedMeshComponent|SetMasterPoseComponent (Variables|Default|GetHead) _skeletalmesh)
  (Class|SkinnedMeshComponent|SetMasterPoseComponent (Variables|Default|GetChest) _skeletalmesh))

(fn SetMesh
  (params (NewStaticMesh :type Static%20Mesh%20Object%20Reference))
  (Components|StaticMesh|SetStaticMesh (Variables|Default|GetViewedMesh) NewStaticMesh)
  (CallFunction|FocusView))

(fn RotateMesh
  (params (RotationDelta :type Rotator) (bLocalSpace :type Boolean))
  (if bLocalSpace
    (Transformation|AddLocalRotation (Variables|Default|GetViewedMesh) RotationDelta false false)
    (else
      (Transformation|AddWorldRotation (Variables|Default|GetViewedMesh) RotationDelta false false))))

(fn SetIsVisible
  (params (NewVisibility :type Boolean))
  (Rendering|SetVisibility (Variables|Default|GetViewedMesh) NewVisibility false))

(fn FocusView
  (bind _viewedmesh (Variables|Default|GetViewedMesh))
  (bind _desiredboundsradius (Variables|Customization|GetDesiredBoundsRadius))
  (bind _maxscale (Variables|Customization|GetMaxScale))
  (bind _sphereradius (Collision|GetComponentBounds _viewedmesh))
  (bind _returnvalue (/ _sphereradius _desiredboundsradius))
  (bind _returnvalue_2 (/ 1.0 _returnvalue))
  (bind _returnvalue_3 (Math|Float|Clamp(Float) _returnvalue_2 0.0 _maxscale))
  (Transformation|SetRelativeScale3D _viewedmesh "1.000000,1.000000,1.000000") ; Reset scale to get correct bounds of new mesh.
  (Transformation|SetRelativeScale3D (Variables|Default|GetViewedMesh) (Math|Vector|MakeVector _returnvalue_3 _returnvalue_3 _returnvalue_3)))