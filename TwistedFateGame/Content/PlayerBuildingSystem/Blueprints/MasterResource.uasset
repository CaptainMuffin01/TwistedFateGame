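; MasterResource is a harvestable resource actor in the player building system, holding an item row and a remaining count.
; Interacting harvests up to two units, adds them to the player's InventoryComponent and updates the client's slot.
; ResourceCollected subtracts the amount and destroys the actor at zero, but returns a smaller remainder without deducting it.
; DeductResource, not called here, is similar but subtracts only when Count is at most the amount.
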(event EventInteract
  (params (Player%20Building%20Component :type Player%20Building%20Component%20Object%20Reference))
  (bind _inventory_component (Variables|/Game/PlayerBuildingSystem/Blueprints/Components/PlayerBuildingComponent.PlayerBuildingComponent_C|GetInventory%20Component Player%20Building%20Component))
  (bind (_item_count _item_name) (CallFunction|ResourceCollected 2))
  (bind _item_out (Default|AddItem _inventory_component (Utilities|Struct|MakeS_Item _item_name _item_count 0 0) false))
  (Default|ClientUpdateInventorySlot _inventory_component _item_out))

(fn ConstructionScript)

(fn ResourceCollected
  (params (Collected%20Amount :type Integer))
  (LocalVariables|SetHarvested%20Amount%20L Collected%20Amount)
  (if (>= (Variables|Default|GetCount) (LocalVariables|GetHarvested%20Amount%20L))
    (if (>= (Variables|Default|GetCount) (LocalVariables|GetHarvested%20Amount%20L))
      (bind _output_get (Variables|Default|SetCount (- (Variables|Default|GetCount) (LocalVariables|GetHarvested%20Amount%20L))))
      (if (> _output_get 0)
        _
        (else
          (Actor|DestroyActor)))
      (return (LocalVariables|GetHarvested%20Amount%20L) (Utilities|String|ToString(Name) (.RowName (Utilities|Struct|BreakDataTableRowHandle (Variables|Default|GetItem))))))
    (else
      (return (Variables|Default|GetCount) (Utilities|String|ToString(Name) (.RowName (Utilities|Struct|BreakDataTableRowHandle (Variables|Default|GetItem))))))))

(fn DeductResource
  (params (Amount :type Integer))
  (LocalVariables|SetAmount%20L Amount)
  (if (<= (Variables|Default|GetCount) (LocalVariables|GetAmount%20L))
    (bind _output_get (Variables|Default|SetCount (- (Variables|Default|GetCount) (LocalVariables|GetAmount%20L))))
    (if (> _output_get 0)
      _
      (else
        (Actor|DestroyActor)))
    (return (Utilities|String|ToString(Name) (.RowName (Utilities|Struct|BreakDataTableRowHandle (Variables|Default|GetItem)))) (LocalVariables|GetAmount%20L))
    (else
      (return (Utilities|String|ToString(Name) (.RowName (Utilities|Struct|BreakDataTableRowHandle (Variables|Default|GetItem)))) (Variables|Default|GetCount)))))