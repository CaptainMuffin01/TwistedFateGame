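; BuildingCharacter is a player character Blueprint that maps keyboard and mouse input to a player building system.
; Each key handler forwards directly to PlayerBuildingComponent, covering mesh rotation, left-click actions, interaction and a demo damage test.
; The build and options menus and the interact action are hold-style inputs, sending true on press and false on release.
; The character holds no building logic itself, and its construction script is empty.
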(event Input|KeyboardEvents|E
  (params (Key :type Key%20Structure))
  ;[1 1 1] Interact input
  (:Pressed
    (Default|ClientInteract (Variables|Components|GetPlayerBuildingComponent) true))
  (:Released
    (Default|ClientInteract (Variables|Components|GetPlayerBuildingComponent) false)))

(event Input|KeyboardEvents|R
  (params (Key :type Key%20Structure))
  ;[1 1 1] Rotate mesh
  (:Pressed
    (Default|RotateMesh (Variables|Components|GetPlayerBuildingComponent))))

(event Input|KeyboardEvents|T
  (params (Key :type Key%20Structure))
  ;[1 1 1] Damage Demo
  (:Pressed
    (Default|ClientDamageTest (Variables|Components|GetPlayerBuildingComponent))))

(event Input|MouseEvents|LeftMouseButton
  (params (Key :type Key%20Structure))
  (bind _playerbuildingcomponent (Variables|Components|GetPlayerBuildingComponent))
  ;[1 1 1] Left mouse button input
  (:Pressed
    (Default|LeftMousePressed _playerbuildingcomponent))
  (:Released
    (Default|LeftMouseReleased _playerbuildingcomponent)))

(event Input|KeyboardEvents|Q
  (params (Key :type Key%20Structure))
  (bind _playerbuildingcomponent (Variables|Components|GetPlayerBuildingComponent))
  ;[1 1 1] Toggle building options menu
  (:Pressed
    (Default|ToggleBuildingOptionsMenu _playerbuildingcomponent true))
  (:Released
    (Default|ToggleBuildingOptionsMenu _playerbuildingcomponent false)))

(event Input|KeyboardEvents|F
  (params (Key :type Key%20Structure))
  (bind _playerbuildingcomponent (Variables|Components|GetPlayerBuildingComponent))
  ;[1 1 1] Toggle building menu
  (:Pressed
    (Default|ToggleBuildMenu _playerbuildingcomponent true))
  (:Released
    (Default|ToggleBuildMenu _playerbuildingcomponent false)))

(fn ConstructionScript)