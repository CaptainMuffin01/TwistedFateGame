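; M4A1 rifle weapon Blueprint that spawns bullets while the player's fire input is held.
; Tick reads AttackFirePressed from the Hero_PC player controller, then calls Fire, which spawns Bullet_BP at the BulletSpawn transform.
; Each pressed tick also resets a non-looping RoundsPerSecond timer, so shots follow frame rate, plus one delayed shot after release.
; The timer-clear and DoOnce reset nodes never run.
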(event Custom|Fire
  (Game|SpawnActorfromClass "/Game/RifleAnimsetPro/Weapons/Bullet_BP.Bullet_BP_C" (Transformation|GetWorldTransform (Variables|Default|GetBulletSpawn)) "Undefined" 0 0))

(event EventTick
  (params (DeltaSeconds :type Float%20%28single-precision%29))
  (bind _ashero_pc (Utilities|Casting|CastToHero_PC (Game|GetPlayerController 0)))
  (Variables|Default|SetAttack/firing (Variables|/Game/RifleAnimsetPro/Survivor/Hero_PC.Hero_PC_C|GetAttack/FirePressed? _ashero_pc))
  (if (Variables|Default|GetAttack/firing)
    (CallFunction|Fire)
    (Utilities|Time|SetTimerbyFunctionName 0 "Fire" (/ 1.0 (Variables|Default|GetRounds%20Per%20Second)))))

(fn ConstructionScript)