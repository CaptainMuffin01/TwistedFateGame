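; Bullet projectile Blueprint that reacts to hits by pushing physics objects and damaging enemies.
; On Hit, a physics-simulating component receives an impulse scaled from the bullet's velocity at its location, then the bullet destroys itself.
; In the same event, hitting an Enemy_BP calls its DamageHealth and destroys the bullet.
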(event Collision|EventHit
  (params (MyComp :type Primitive%20Component%20Object%20Reference) (Other :type Actor%20Object%20Reference) (OtherComp :type Primitive%20Component%20Object%20Reference) (bSelfMoved :type Boolean) (HitLocation :type Vector :default "0, 0, 0") (HitNormal :type Vector :default "0, 0, 0") (NormalImpulse :type Vector :default "0, 0, 0") (Hit :type Hit%20Result%20Structure%20%28by%20ref%29))
  (Utilities|FlowControl|Sequence
    (:then_0
      (if (Physics|IsSimulatingPhysics OtherComp "None")
        (Physics|AddImpulseatLocation OtherComp (* (Transformation|GetVelocity) 1e+02) (Transformation|GetActorLocation) "None")
        (Actor|DestroyActor)))
    (:then_1
      (bind _asenemy_bp (Utilities|Casting|CastToEnemy_BP Other))
      (Default|DamageHealth _asenemy_bp)
      (Actor|DestroyActor))))

(fn ConstructionScript)