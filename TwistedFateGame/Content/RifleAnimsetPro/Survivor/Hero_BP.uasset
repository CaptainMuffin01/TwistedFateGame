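; Player character for a third-person shooter with building, handling movement, aiming, health and building input.
; BeginPlay attaches an M4A1 to the rifle socket and adds health bar and blood effect widgets.
; AnyDamage lowers health and plays a death animation at zero, while Tick applies regeneration and refreshes the health bar.
; Aim toggles ADS through server events, changing walk speed and spring arm length, and build keys forward to PlayerBuildingComponent.
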(event Custom|CheckHP
  ;[1 1 1] Checking for Death *Might Not Need*
)

(event Custom|ServerStartADS
  ;[1 1 1] Camera Zoom When Aiming Down Sights
  (Weapons|StartADS))

(event Custom|ServerStopADS
  ;[1 1 1] Camera Zoom When Aiming Down Sights
  (Weapons|StopADS))

(event EventBeginPlay
  (bind _mesh (Variables|Character|GetMesh))
  (Utilities|FlowControl|Sequence
    (:then_0
      ;[1 1 1] M4 Hand Socket
      (bind _returnvalue (Game|SpawnActorfromClass "/Game/RifleAnimsetPro/Weapons/M4A1_BP.M4A1_BP_C" (Transformation|GetSocketTransform _mesh "RifleSocket" "RTS_World") "Undefined" 0 0))
      (bind _output_get (Variables|Components|SetM4A1_BP _returnvalue))
      (Transformation|AttachComponentToComponent _output_get _mesh "RifleSocket" "SnapToTarget" "SnapToTarget" "SnapToTarget" true))
    (:then_1
      ;[1 1 1] HealthBar to Viewport
      (bind _returnvalue_2 (UserInterface|CreateWidget "/Game/RifleAnimsetPro/Widgets/HealthBar.HealthBar_C"))
      (bind _output_get_2 (Variables|Components|SetHealthBarWidget _returnvalue_2))
      (UserInterface|Viewport|AddtoViewport _output_get_2 0))
    (:then_2
      ;[1 1 1] Event Damage W/ BloodAffect
      (bind _returnvalue_3 (UserInterface|CreateWidget "/Game/RifleAnimsetPro/Widgets/BloodEffect.BloodEffect_C"))
      (bind _output_get_3 (Variables|Default|SetBloodEffectReference _returnvalue_3))
      (UserInterface|Viewport|AddtoViewport _output_get_3 0))))

(event EventTick
  (params (DeltaSeconds :type Float%20%28single-precision%29))
  (Utilities|FlowControl|Sequence
    (:then_0
      (CallFunction|UpdateHealth 0 0.0))))

(event Game|Damage|EventAnyDamage
  (params (Damage :type Float%20%28single-precision%29) (DamageType :type Damage%20Type%20Object%20Reference) (InstigatedBy :type Controller%20Object%20Reference) (DamageCauser :type Actor%20Object%20Reference))
  ;[1 1 1] Event Damage W/ BloodAffect
  (bind _output_get (Variables|Default|SetCurrent%20health (- (Variables|Default|GetCurrent%20health) Damage)))
  (Default|CallUpdateHealthDispatch _output_get)
  (if (<= (Variables|Default|GetCurrent%20health) 0.0)
    (Components|Animation|PlayAnimation (Variables|Character|GetMesh) "/Game/RifleAnimsetPro/Animations/RootMotion/Rifle_Death_3.Rifle_Death_3" false)))

(event Input|ActionEvents|InputActionSelect
  (params (Key :type Key%20Structure))
  (bind _playerbuildingcomponent (Variables|Default|GetPlayerBuildingComponent))
  ;[1 1 1] BuildingSystem
  ;;[1 1 1] Left mouse button input
  (:Pressed
    (Default|LeftMousePressed _playerbuildingcomponent))
  (:Released
    (Default|LeftMouseReleased _playerbuildingcomponent)))

(event Input|ActionEvents|InputActionAim
  (params (Key :type Key%20Structure))
  (bind _cameraspringarm (Variables|Default|GetCameraSpringArm))
  (bind _charactermovement (Variables|Character|GetCharacterMovement))
  ;[1 1 1] Camera Zoom When Aiming Down Sights
  (:Pressed
    (Variables|/Script/Engine.CharacterMovementComponent|SetMaxWalkSpeed _charactermovement 2e+02)
    (Weapons|ToggleADS :!label _label)
    (if (Variables|Default|GetIsADS)
      (Variables|/Script/Engine.SpringArmComponent|SetTargetArmLength _cameraspringarm 1e+02)
      (else
        (Variables|/Script/Engine.SpringArmComponent|SetTargetArmLength _cameraspringarm 1.7e+02))))
  (:Released
    (Variables|/Script/Engine.CharacterMovementComponent|SetMaxWalkSpeed _charactermovement 4e+02)
    (goto _label)))

(event Input|AxisEvents|InputAxisMoveRight
  (params (AxisValue :type Float%20%28single-precision%29))
  ;[1 1 1] WorldMovement
  (bind _ashero_pc (Utilities|Casting|CastToHero_PC (Game|GetPlayerController 0)))
  (Variables|Default|SetSprint%20Pressed (Variables|/Game/RifleAnimsetPro/Survivor/Hero_PC.Hero_PC_C|GetSprintingpressed? _ashero_pc))
  (Variables|Default|SetProne%20Pressed? (Variables|/Game/RifleAnimsetPro/Survivor/Hero_PC.Hero_PC_C|GetProne%20Pressed? _ashero_pc))
  (if (not (or (Variables|Default|GetSprint%20Pressed) (Variables|Default|GetProne%20Pressed?)))
    (Pawn|Input|AddMovementInput (Math|Vector|GetRightVector (Math|Rotator|MakeRotator 0.0 0.0 (.Yaw (Math|Rotator|BreakRotator (Pawn|GetControlRotation (Game|GetPlayerController 0) :!class /Script/Engine.Controller))))) AxisValue false)))

(event Input|AxisEvents|InputAxisMoveForward
  (params (AxisValue :type Float%20%28single-precision%29))
  ;[1 1 1] WorldMovement
  (if (not (Variables|Default|GetDisable%20Movement))
    (Pawn|Input|AddMovementInput (Math|Vector|GetForwardVector (Math|Rotator|MakeRotator 0.0 0.0 (.Yaw (Math|Rotator|BreakRotator (Pawn|GetControlRotation (Game|GetPlayerController 0) :!class /Script/Engine.Controller))))) AxisValue false)))

(event Input|KeyboardEvents|E
  (params (Key :type Key%20Structure))
  ;[1 1 1] BuildingSystem
  ;;[1 1 1] Interact input
  (:Pressed
    (Default|ClientInteract (Variables|Default|GetPlayerBuildingComponent) true))
  (:Released
    (Default|ClientInteract (Variables|Default|GetPlayerBuildingComponent) false)))

(event Input|KeyboardEvents|T
  (params (Key :type Key%20Structure))
  ;[1 1 1] BuildingSystem
  ;;[1 1 1] Damage Demo
  (:Pressed
    (Default|ClientDamageTest (Variables|Default|GetPlayerBuildingComponent))))

(event Input|KeyboardEvents|C
  (params (Key :type Key%20Structure))
  (bind _playerbuildingcomponent (Variables|Default|GetPlayerBuildingComponent))
  ;[1 1 1] BuildingSystem
  ;;[1 1 1] Toggle building menu
  (:Pressed
    (Default|ToggleBuildMenu _playerbuildingcomponent true))
  (:Released
    (Default|ToggleBuildMenu _playerbuildingcomponent false)))

(event Input|KeyboardEvents|V
  (params (Key :type Key%20Structure))
  ;[1 1 1] BuildingSystem
  ;;[1 1 1] Rotate mesh
  (:Pressed
    (Default|RotateMesh (Variables|Default|GetPlayerBuildingComponent))))

(event Input|KeyboardEvents|Q
  (params (Key :type Key%20Structure))
  (bind _playerbuildingcomponent (Variables|Default|GetPlayerBuildingComponent))
  ;[1 1 1] BuildingSystem
  ;;[1 1 1] Toggle building options menu
  (:Pressed
    (Default|ToggleBuildingOptionsMenu _playerbuildingcomponent true))
  (:Released
    (Default|ToggleBuildingOptionsMenu _playerbuildingcomponent false)))

(fn ConstructionScript)

(fn UpdateHealth
  (params (Damage :type Integer) (Health :type Float%20%28single-precision%29))
  (bind _max_health (Variables|Default|GetMax%20Health))
  (if (<= (Variables|Default|GetCurrent%20health) (Variables|Default|GetMax%20Health))
    (bind _output_get (Variables|Default|SetCurrent%20health (+ (Variables|Default|GetCurrent%20health) (* (/ (Utilities|Time|GetWorldDeltaSeconds) 5e+01) (Variables|Default|GetRegenHealth)))))
    (Default|CallUpdateHealthDispatch _output_get)
    (bind _ashealth_bar (Utilities|Casting|CastToHealthBar (Variables|Components|GetHealthBarWidget)))
    (Variables|/Game/RifleAnimsetPro/Widgets/HealthBar.HealthBar_C|SetHealthPercentage _ashealth_bar (/ (Variables|Default|GetCurrent%20health) _max_health))
    (Variables|/Game/RifleAnimsetPro/Widgets/HealthBar.HealthBar_C|SetHealth%20Text _ashealth_bar (Utilities|String|Append (Utilities|String|Append (Utilities|String|ToString(Integer) (Math|Float|Floor (Variables|Default|GetCurrent%20health))) "/") (Utilities|String|ToString(Integer) (Math|Float|Floor _max_health))))))

(fn ToggleADS
  (if (Variables|Default|GetIsADS)
    (Weapons|StopADS)
    (else
      (Weapons|StartADS))))

(fn StartADS
  (Networking|SwitchHasAuthority
    (:Authority
      _)
    (:Remote
      (CallFunction|ServerStartADS)))
  (Variables|Default|SetIsADS true))

(fn StopADS
  (Networking|SwitchHasAuthority
    (:Authority
      _)
    (:Remote
      (CallFunction|ServerStopADS)))
  (Variables|Default|SetIsADS false))