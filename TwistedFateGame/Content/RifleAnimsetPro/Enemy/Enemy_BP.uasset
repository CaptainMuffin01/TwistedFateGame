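; Enemy pawn that chases the player and self-destructs on arrival, with no damage dealt in this graph.
; BeginPlay calls ChasePlayer, which runs AI MoveTo toward the player and, on success, spawns explosion particles and sound, re-calls itself, then destroys the actor.
; A Roam event is never called and also targets the player, leaving its random navigable point node unconnected.
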(event Custom|ChasePlayer
  (bind _self self)
  (bind _returnvalue (Transformation|GetActorLocation _self))
  (AI|AIMoveTo _self "0, 0, 0" (Game|GetPlayerCharacter 0) 5.0 false
    (:OnSuccess
      (Effects|SpawnEmitteratLocation "/Game/StarterContent/Particles/P_Explosion.P_Explosion" _returnvalue)
      (Audio|PlaySoundatLocation "/Game/StarterContent/Audio/Explosion_Cue.Explosion_Cue" _returnvalue)
      (CallFunction|ChasePlayer)
      (Actor|DestroyActor))))

(event Custom|Roam
  (AI|AIMoveTo self "0, 0, 0" (Game|GetPlayerCharacter 0) 5.0 false
    (:OnSuccess
      (CallFunction|Roam))))

(event EventBeginPlay
  (Utilities|FlowControl|Sequence
    (:then_0
      (CallFunction|ChasePlayer))))

(fn ConstructionScript)